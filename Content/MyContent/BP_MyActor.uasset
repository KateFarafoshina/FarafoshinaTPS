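; BP_MyActor is an actor Blueprint that appears to exercise functions and variables inherited from its parent class through debug printing.
; Its ChangeSpeed override calls the parent version, scales the result by 1000, then prints and returns it.
; BeginPlay and MyPrintHP are empty.
; The EventGraph chains that print speed, test AreNumbersEqual and set HP from MaxHP are disconnected, so they never run.
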(event `self.MyPrintHP`)

(event `self.ReceiveBeginPlay`)

(fn `ChangeSpeed`
  (params (MoveSpeed :type Integer))
  (returns (ReturnValue :type Integer))
  (bind _returnvalue (`parent.ChangeSpeed` MoveSpeed))
  (bind _returnvalue_2 (* _returnvalue 1000))
  (`KismetSystemLibrary.PrintString` (`KismetStringLibrary.Conv_IntToString` _returnvalue_2) true true (struct :`G` 0.66 :`B` 1.0 :`A` 1.0) 20.0)
  (return _returnvalue_2))

(fn `UserConstructionScript`)