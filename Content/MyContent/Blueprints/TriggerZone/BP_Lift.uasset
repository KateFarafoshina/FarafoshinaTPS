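; BP_Lift is a trigger-driven lift actor that rises 500 units along Z from its starting location.
; BeginPlay caches the start and raised end positions.
; Beginning an overlap with its Box component plays the Lift timeline, which lerps the actor between those positions without sweeping, and ending an overlap reverses it to lower the lift.
; Overlaps are not filtered by actor.
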(event `self.ReceiveBeginPlay`
  (bind _returnvalue (`self.K2_GetActorLocation`))
  (set `self.Start` _returnvalue)
  (set `self.End` (+ _returnvalue (0.0 0.0 500.0))))

(event `self.Box.OnComponentBeginOverlap`
  (params (OverlappedComponent :type "PrimitiveComponent Object Reference") (OtherActor :type "Actor Object Reference") (OtherComp :type "PrimitiveComponent Object Reference") (OtherBodyIndex :type Integer) (bFromSweep :type Boolean) (SweepResult :type "HitResult Structure (by ref)"))
  (bind (_direction _lift) (`Timeline|Lift` :!label _label)
    (:`Update`
      (`self.K2_SetActorLocation` (`KismetMathLibrary.VLerp` (`self.Start`) (`self.End`) _lift)))))

(event `self.Box.OnComponentEndOverlap`
  (params (OverlappedComponent :type "PrimitiveComponent Object Reference") (OtherActor :type "Actor Object Reference") (OtherComp :type "PrimitiveComponent Object Reference") (OtherBodyIndex :type Integer))
  (goto _label :!via `Reverse`))

(fn `UserConstructionScript`)