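; BP_TriggerZone is a traffic light trigger: overlaps cycle through red, yellow and green, ignored with a printed message while one is lit.
; CountEntries tallies entries; LightChange picks the light from count modulo three, taking color, name and duration from DT_TrafficLighters.
; Timers switch the light off and tick a countdown to WBPInfo, but the looping countdowns are never cleared.
; The WBP_Info creation chain is unconnected, so WBPInfo is never assigned here.
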(event `RedLight`
  (`LightComponent.SetIntensity` (`self.Red`) 0.0)
  (set `self.IsActive` false))

(event `StartTimer`
  (bind _result (`/Engine/EditorBlueprintResources/StandardMacros.DecrementFloat` (`self.Timer`))
    (:`  `
      (`/Game/MyContent/Widget/WBP_Info.UpdateTimer` (`self.WBP_Info`) _result))))

(event `self.Box.OnComponentBeginOverlap`
  (params (OverlappedComponent :type "PrimitiveComponent Object Reference") (OtherActor :type "Actor Object Reference") (OtherComp :type "PrimitiveComponent Object Reference") (OtherBodyIndex :type Integer) (bFromSweep :type Boolean) (SweepResult :type "HitResult Structure (by ref)"))
  (bind _wbp_info (`self.WBP_Info`))
  (bind _wbp_info_2 (`self.WBP_Info`))
  (bind _yellow (`self.Yellow`))
  (bind _green (`self.Green`))
  (bind _red (`self.Red`))
  (bind _wbp_info_3 (`self.WBP_Info`))
  (if (`self.IsActive`)
    (`KismetSystemLibrary.PrintString` "Светофор уже горит!")
    (else
      (bind _output_get (`self.CountEntries`))
      (`self.LightChange` (mod _output_get 3)
        (:`Red`
          (bind _returnvalue (`|GetDataTableRow` "/Game/MyContent/StructuresAndDataTables/DT_TrafficLighters.DT_TrafficLighters" "RedLight")
            (:`then`
              (set `self.IsActive` true)
              (bind (_name _color _timer) (break `/Game/MyContent/StructuresAndDataTables/ST_Light` _returnvalue))
              (set `self.Timer` _timer)
              (`LightComponent.SetLightColor` _red (`KismetMathLibrary.Conv_ColorToLinearColor` _color) true)
              (`LightComponent.SetIntensity` _red 5000.0)
              (`/Game/MyContent/Widget/WBP_Info.UpdateTimer` _wbp_info_3 (`self.Timer`))
              (`/Game/MyContent/Widget/WBP_Info.UpdateColor` _wbp_info_3 _name)
              (`KismetSystemLibrary.K2_SetTimerDelegate` (delegate `RedLight`) (`self.Timer`))
              (`KismetSystemLibrary.K2_SetTimerDelegate` (delegate `StartTimer`) 1.0 true))))
        (:`Yellow`
          (bind _returnvalue_2 (`|GetDataTableRow` "/Game/MyContent/StructuresAndDataTables/DT_TrafficLighters.DT_TrafficLighters" "YellowLight")
            (:`then`
              (set `self.IsActive` true)
              (bind (_name_2 _color_2 _timer_2) (break `/Game/MyContent/StructuresAndDataTables/ST_Light` _returnvalue_2))
              (set `self.Timer` _timer_2)
              (`LightComponent.SetLightColor` _yellow (`KismetMathLibrary.Conv_ColorToLinearColor` _color_2) true)
              (`LightComponent.SetIntensity` _yellow 5000.0)
              (`/Game/MyContent/Widget/WBP_Info.UpdateTimer` _wbp_info_2 (`self.Timer`))
              (`/Game/MyContent/Widget/WBP_Info.UpdateColor` _wbp_info_2 _name_2)
              (`KismetSystemLibrary.K2_SetTimerDelegate` (delegate `YellowLight`) (`self.Timer`))
              (`KismetSystemLibrary.K2_SetTimerDelegate` (delegate `StartTimerYellow`) 1.0 true))))
        (:`Green`
          (bind _returnvalue_3 (`|GetDataTableRow` "/Game/MyContent/StructuresAndDataTables/DT_TrafficLighters.DT_TrafficLighters" "GreenLight")
            (:`then`
              (set `self.IsActive` true)
              (bind (_name_3 _color_3 _timer_3) (break `/Game/MyContent/StructuresAndDataTables/ST_Light` _returnvalue_3))
              (set `self.Timer` _timer_3)
              (`LightComponent.SetLightColor` _green (`KismetMathLibrary.Conv_ColorToLinearColor` _color_3) true)
              (`LightComponent.SetIntensity` _green 5000.0)
              (`/Game/MyContent/Widget/WBP_Info.UpdateTimer` _wbp_info (`self.Timer`))
              (`/Game/MyContent/Widget/WBP_Info.UpdateColor` _wbp_info _name_3)
              (`KismetSystemLibrary.K2_SetTimerDelegate` (delegate `GreenLight`) (`self.Timer`))
              (`KismetSystemLibrary.K2_SetTimerDelegate` (delegate `StartTimerGreen`) 1.0 true))))))))

(event `self.ReceiveBeginPlay`)

(event `YellowLight`
  (`LightComponent.SetIntensity` (`self.Yellow`) 0.0)
  (set `self.IsActive` false))

(event `StartTimerYellow`
  (bind _result (`/Engine/EditorBlueprintResources/StandardMacros.DecrementFloat` (`self.Timer`))
    (:`  `
      (`/Game/MyContent/Widget/WBP_Info.UpdateTimer` (`self.WBP_Info`) _result))))

(event `GreenLight`
  (`LightComponent.SetIntensity` (`self.Green`) 0.0)
  (set `self.IsActive` false))

(event `StartTimerGreen`
  (bind _result (`/Engine/EditorBlueprintResources/StandardMacros.DecrementFloat` (`self.Timer`))
    (:`  `
      (`/Game/MyContent/Widget/WBP_Info.UpdateTimer` (`self.WBP_Info`) _result))))

(fn `UserConstructionScript`)